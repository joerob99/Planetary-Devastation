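; BP_ResourcePlanet is a planet actor that tracks the resources and aliens around it through its PlanetResourceComp.
; On BeginPlay it seeds the component's lists from actors overlapping its Sphere and starts an interval growth loop.
; Overlap events add or remove resources, though a note flags removal as unreliable pending an inventory hookup.
; The construction script applies the atmosphere material and scale and sets the Sphere to the gravity field radius.
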(event EventBeginPlay
  (bind _planetresourcecomp (Variables|Default|GetPlanetResourceComp))
  (bind _sphere (Variables|Default|GetSphere))
  (Class|PlanetResourceComponent|InitializeResourceList _planetresourcecomp (Collision|GetOverlappingActors _sphere "/Game/Blueprints/ResourceSystem/BP_Resource.BP_Resource_C" :!class /Script/Engine.PrimitiveComponent))
  (Class|PlanetResourceComponent|InitializeAlienList _planetresourcecomp (Collision|GetOverlappingActors _sphere "/Game/Blueprints/BP_Alien.BP_Alien_C" :!class /Script/Engine.PrimitiveComponent))
  (Class|PlanetResourceComponent|IntervalGrowthLoop _planetresourcecomp))

(event Collision|EventActorBeginOverlap
  (params (OtherActor :type Actor%20Object%20Reference))
  (if (== (Utilities|GetClass OtherActor) "/Game/Blueprints/ResourceSystem/BP_Resource.BP_Resource_C")
    (Class|PlanetResourceComponent|AddResource (Variables|Default|GetPlanetResourceComp) OtherActor)))

(event EventTick
  (params (DeltaSeconds :type Float%20%28single-precision%29))
  ;[1 1 1] Debug
)

(event Collision|EventActorEndOverlap
  (params (OtherActor :type Actor%20Object%20Reference))
  (if (== (Utilities|GetClass OtherActor) "/Game/Blueprints/ResourceSystem/BP_Resource.BP_Resource_C")
    (Class|PlanetResourceComponent|RemoveResource (Variables|Default|GetPlanetResourceComp) OtherActor)))

(fn ConstructionScript
  (bind _atmosphere (Variables|Default|GetAtmoSphere))
  (|CallParentFunction)
  (Rendering|Material|SetMaterial _atmosphere 0 (Variables|AtmoSphere|GetAtmoSphereMaterial))
  (Transformation|SetRelativeScale3D _atmosphere (Variables|AtmoSphere|GetAtmoSphereScale))
  (Components|Sphere|SetSphereRadius (Variables|Default|GetSphere) (Variables|AtmoSphere|GetGravityFieldRadius) true))