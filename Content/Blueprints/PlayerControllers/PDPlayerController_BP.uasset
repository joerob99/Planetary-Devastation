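; PDPlayerController_BP is a player controller that puts the HUD on screen and opens the pause menu.
; BeginPlay creates the HUD widget, stores it in HudWidget and adds it to the viewport.
; Tab adds the existing PauseMenu widget at Z-order 100 if it is not already shown; this graph neither creates nor removes that widget, nor pauses the game.
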(event EventBeginPlay
  (|CallParentFunction)
  (bind _returnvalue (UserInterface|CreateWidget "/Game/InventorySystem/inventoryUi/HUD.HUD_C"))
  (bind _output_get (Variables|Default|SetHud_Widget _returnvalue))
  (UserInterface|Viewport|AddtoViewport _output_get 0))

(event EventTick
  (params (DeltaSeconds :type Float%20%28single-precision%29))
  (|CallParentFunction 0.0))

(event Input|KeyboardEvents|Tab
  (params (Key :type Key%20Structure :default "None"))
  (bind _pausemenu (Variables|Default|GetPauseMenu))
  (:Pressed
    (if (not (UserInterface|Viewport|IsinViewport _pausemenu))
      (UserInterface|Viewport|AddtoViewport _pausemenu 100))))

(fn ConstructionScript)