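; BP_ResourcePlanet is a planet actor that tracks the BP_Resource actors on or around it through its PlanetResourceComp.
; On BeginPlay it seeds the component's resource list from the resources overlapping its Sphere.
; Actor begin and end overlaps then add or remove resources of exactly that class.
; The removal path is flagged as unreliable, with an inventory-system event noted as the intended replacement.
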(event EventBeginPlay
  (Class|PlanetResourceComponent|InitializeResourceList (Variables|Default|GetPlanetResourceComp) (Collision|GetOverlappingActors (Variables|Default|GetSphere) "/Game/ResourceSystem/BP_Resource.BP_Resource_C" :!class /Script/Engine.PrimitiveComponent)))

(event Collision|EventActorBeginOverlap
  (params (OtherActor :type Actor%20Object%20Reference))
  (if (== (Utilities|GetClass OtherActor) "/Game/ResourceSystem/BP_Resource.BP_Resource_C")
    (Class|PlanetResourceComponent|AddResource (Variables|Default|GetPlanetResourceComp) OtherActor)))

(event EventTick
  (params (DeltaSeconds :type Float%20%28single-precision%29)))

(event Collision|EventActorEndOverlap
  (params (OtherActor :type Actor%20Object%20Reference))
  (if (== (Utilities|GetClass OtherActor) "/Game/ResourceSystem/BP_Resource.BP_Resource_C")
    (Class|PlanetResourceComponent|RemoveResource (Variables|Default|GetPlanetResourceComp) OtherActor)))

(fn ConstructionScript
  (|CallParentFunction))