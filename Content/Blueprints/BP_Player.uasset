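; Player character Blueprint handling the screen UI, inventory toggle, sprinting, key-driven hunger adjustment and a summonable UFO.
; Camera line traces drive interface-based interaction and placing of items from the selected inventory slot, decrementing its quantity.
; Summoning spawns a UFO above the player, or replaces the existing one after particles and a distance-scaled logarithmic delay.
; The looping trace timer started on BeginPlay calls an empty event.
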(event Custom|CustomEvent_0
  ;[1 1 1] trace actor(get whatever actor camera pointing at
)

(event EventBeginPlay
  ;[1 1 1] user interface
  (Game|GetCurrentLevelName true)
  (bind _returnvalue (UserInterface|CreateWidget "/Game/screenUi/screenUi.screenUi_C"))
  (UserInterface|Viewport|AddtoViewport _returnvalue 0)
  (|CallParentFunction)
  (Utilities|FlowControl|Sequence
    (:then_0
      ;[1 1 1] set up  summon variables
      (bind _outactors (Actor|GetAllActorsOfClass "/Game/Blueprints/BP_UFO.BP_UFO_C"))
      (Variables|Default|SetUFOisSummoned (Utilities|IsValid (Utilities|Array|Get(acopy) _outactors)))
      (if (Utilities|IsValid (Utilities|Array|Get(acopy) _outactors))
        (Variables|Default|SetUFOPawn (Utilities|Array|Get(acopy) _outactors))))
    (:then_1
      ;[1 1 1] trace actor(get whatever actor camera pointing at
      (Utilities|Time|SetTimerbyEvent (delegate Custom|CustomEvent_0) 0.1 true))))

(event Input|ActionEvents|InputActioninventory
  (params (Key :type Key%20Structure :default "None"))
  ;[1 1 1] toggle inventory
  (:Pressed
    (Default|ToggleInventory (Variables|Default|GetinventoryComponenet))))

(event Input|ActionEvents|InputActionSprint
  (params (Key :type Key%20Structure :default "None"))
  (bind _charactermovement (Variables|Character|GetCharacterMovement))
  ;[1 1 1] Sprint Logic
  (:Pressed
    (Variables|Default|SetSprinting true)
    (Variables|/Script/Engine.CharacterMovementComponent|SetMaxWalkSpeed _charactermovement (* (Variables|/Script/Engine.CharacterMovementComponent|GetMaxWalkSpeed _charactermovement) 2.0)))
  (:Released
    (Variables|Default|SetSprinting false)
    (Variables|/Script/Engine.CharacterMovementComponent|SetMaxWalkSpeed _charactermovement (/ (Variables|/Script/Engine.CharacterMovementComponent|GetMaxWalkSpeed _charactermovement) 2.0))))

(event Input|ActionEvents|InputActioninteract
  (params (Key :type Key%20Structure :default "None"))
  (bind _camera (Variables|Default|GetCamera))
  (bind _returnvalue (Transformation|GetWorldLocation _camera))
  ;[1 1 1] trace actor(get whatever actor camera pointing at
  (:Pressed
    (bind _outhit (Collision|LineTraceByChannel _returnvalue (+ _returnvalue (* (Math|Vector|GetForwardVector _camera) (Variables|Default|GetInteractRange))) "TraceTypeQuery1" false 0 "None"))
    ;[1 1 1] interact with said actor
    (if (Utilities|DoesObjectImplementInterface (.hitactor _outhit) "/Game/InventorySystem/interact_interface.interact_interface_C")
      (Class|InteractInterface|Interact(Message) (.hitactor _outhit) self))))

(event Input|ActionEvents|InputActionSummonUFO
  (params (Key :type Key%20Structure :default "None"))
  (bind _self self)
  (bind _returnvalue (Transformation|GetActorRotation _self))
  (bind _returnvalue_2 (Transformation|GetActorLocation _self))
  (bind _returnvalue_3 (Math|Transform|MakeTransform _returnvalue_2 _returnvalue "4.000000,4.000000,3.400000"))
  ;[1 1 1] Summon UFO
  (:Released
    (if (Variables|Default|GetUFOisSummoned)
      (bind _returnvalue_4 (Effects|SpawnEmitteratLocation "/Game/WarpsPack/Warps/SimpleWarp/P_SimpleStars.P_SimpleStars" _returnvalue_2 _returnvalue))
      (Utilities|FlowControl|Delay (* (Math|Float|Log (* (Math|Vector|Distance(Vector) (Transformation|GetActorLocation self) (Transformation|GetActorLocation (Variables|Default|GetUFOPawn))) 0.0005) 1e+01) (* (Math|Vector|Distance(Vector) (Transformation|GetActorLocation self) (Transformation|GetActorLocation (Variables|Default|GetUFOPawn))) 0.0005)))
      (Components|DestroyComponent _returnvalue_4)
      (Actor|DestroyActor (Variables|Default|GetUFOPawn))
      (bind _returnvalue_5 (Game|SpawnActorfromClass "/Game/Blueprints/BP_UFO.BP_UFO_C" _returnvalue_3 "AdjustIfPossibleButAlwaysSpawn" 0 0))
      (bind _output_get (Variables|Default|SetUFOPawn _returnvalue_5))
      (Transformation|AddActorLocalOffset _output_get "0,0.000000,370.000000" false false)
      (else
        (bind _returnvalue_6 (Game|SpawnActorfromClass "/Game/Blueprints/BP_UFO.BP_UFO_C" _returnvalue_3 "AdjustIfPossibleButAlwaysSpawn" 0 0))
        (bind _output_get_2 (Variables|Default|SetUFOPawn _returnvalue_6))
        (Transformation|AddActorLocalOffset _output_get_2 "0,0.000000,370.000000" false false)
        (Variables|Default|SetUFOisSummoned true)))))

(event Input|ActionEvents|InputActionPlaceItem
  (params (Key :type Key%20Structure :default "None"))
  (bind _camera (Variables|Default|GetCamera))
  (bind _currslot (Variables|Default|GetcurrSlot))
  (bind _inventorycomponenet (Variables|Default|GetinventoryComponenet))
  (bind _returnvalue (Transformation|GetWorldLocation _camera))
  (bind _slotindex (Variables|/Game/InventorySystem/inventoryUi/inventorySlot.inventorySlot_C|GetSlotIndex _currslot))
  (bind _inventory (Variables|/Game/InventorySystem/inventoryComponenet.inventoryComponenet_C|Getinventory _inventorycomponenet))
  (bind _output (Utilities|Array|Get(acopy) _inventory _slotindex))
  (bind _output_2 (Utilities|Array|Get(acopy) _inventory _slotindex))
  ;[1 1 1] Handle placing items from inventory and updating their values in the inventory slot
  (:Pressed
    (bind _outhit (Collision|LineTraceByChannel _returnvalue (+ _returnvalue (* (Math|Vector|GetForwardVector _camera) 1250)) "TraceTypeQuery1" false 0 "None"))
    (if (Utilities|IsValid _currslot)
      (if (.bblockinghit _outhit)
        (if (.placeable (.itemstruture _output))
          (if (> (.quantity _output) 0)
            (Utilities|Array|SetArrayElem _inventory _slotindex (Utilities|Struct|MakeslotStructure (.itemstruture _output_2) (- (.quantity _output_2) 1)))
            (Game|SpawnActorfromClass (.class (.itemstruture _output)) (Math|Transform|MakeTransform (.location _outhit) (Transformation|GetWorldRotation (Variables|Default|GetCapsuleComponent))) "AdjustIfPossibleButAlwaysSpawn" 0 0)
            (Default|Resfresh (Variables|Default|GetcurrSlot))))))))

(event Input|KeyboardEvents|Down
  (params (Key :type Key%20Structure :default "None"))
  ;[1 1 1] substract hunger
  (:Pressed
    (Variables|Default|Sethunger (Math|Float|Clamp(Float) (- (Variables|Default|Gethunger) 1e+01) 0.0 (Variables|Default|GetmaxHunger)))))

(event Input|KeyboardEvents|Up
  (params (Key :type Key%20Structure :default "None"))
  ;[1 1 1] add hunger
  (:Pressed
    (Variables|Default|Sethunger (Math|Float|Clamp(Float) (+ (Variables|Default|Gethunger) 1e+01) 0.0 (Variables|Default|GetmaxHunger)))))

(fn ConstructionScript
  (|CallParentFunction))